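; BP_Timer is a utility countdown timer actor that broadcasts its progress and completion.
; StartTimer resets CurrentTime to MaxTime and enables actor tick at TimeInterval, using tick instead of timer handles.
; Each tick reports and decrements the remaining time until zero, despite the "elapsed" naming of the event and getter.
; StopTimer disables tick and fires the finished event, so stopping early also signals completion.
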(event Custom|Start%20Timer
  (Variables|Internal|SetCurrent%20Time (Variables|Settings|GetMax%20Time))
  (Actor|Tick|SetActorTickInterval (Variables|Settings|GetTime%20Interval))
  (Actor|Tick|SetActorTickEnabled true))

(event Custom|Stop%20Timer
  (Actor|Tick|SetActorTickEnabled false)
  (Default|CallOnTimerFinished))

(event EventBeginPlay)

(event EventTick
  (params (DeltaSeconds :type Float%20%28single-precision%29))
  (if (<= (Variables|Internal|GetCurrent%20Time) 0.0)
    (CallFunction|StopTimer)
    (else
      (bind _output_get (Variables|Internal|SetCurrent%20Time (- (Variables|Internal|GetCurrent%20Time) DeltaSeconds)))
      (Default|CallOnTimeElapsedEvent _output_get))))

(fn ConstructionScript)

(fn GetCurrentTimeElapsed
  (return (Variables|Internal|GetCurrent%20Time)))