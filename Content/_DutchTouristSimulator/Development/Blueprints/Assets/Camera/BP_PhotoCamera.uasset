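; BP_PhotoCamera is a photo camera actor that the game can raise, lower and use to take pictures.
; Aim and idle events snap a Plane between raised and lowered relative Z positions, using lerps fixed at full alpha.
; MakePicture waits briefly, then draws the camera screen material into the next render target in an array, advancing a counter.
; ResetPictures, also run on BeginPlay, clears every target and zeroes that counter.
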(event Custom|MakePicture
  (bind _count (Variables|Default|GetCount))
  ;[1 1 1] Add picture to texture.
  (Utilities|FlowControl|Delay 0.2)
  (Rendering|DrawMaterialtoRenderTarget (Utilities|Array|Get(acopy) (Variables|Default|GetTexture%20Render%20Target) _count) "/Game/_DutchTouristSimulator/Development/Blueprints/Assets/Camera/CameraTexturesMaterials/M_MainCameraScreen.M_MainCameraScreen")
  (Math|Integer|IncrementInt _count))

(event Custom|ResetPictures
  ;[1 1 1] Reset all textures
  (for _array_element (Variables|Default|GetTexture%20Render%20Target)
    (Rendering|ClearRenderTarget2D _array_element "(R=1.000000,G=1.000000,B=1.000000,A=0.000000)"))
  (Variables|Default|SetCount 0))

(event Custom|AimTheCamera
  (bind _plane (Variables|Default|GetPlane))
  (bind _relativelocation (Variables|/Script/Engine.SceneComponent|GetRelativeLocation _plane))
  ;[1 1 1] Camera move in to screen
  (Transformation|SetRelativeLocation (Variables|Default|GetPlane) (Math|Vector|Lerp(Vector) (Variables|/Script/Engine.SceneComponent|GetRelativeLocation _plane) (Math|Vector|MakeVector (.x _relativelocation) (.y _relativelocation) 0.0) 1.0) false false))

(event Custom|IdleTheCamera
  (bind _plane (Variables|Default|GetPlane))
  (bind _relativelocation (Variables|/Script/Engine.SceneComponent|GetRelativeLocation _plane))
  ;[1 1 1] Camera move out of screen
  (Transformation|SetRelativeLocation (Variables|Default|GetPlane) (Math|Vector|Lerp(Vector) (Variables|/Script/Engine.SceneComponent|GetRelativeLocation _plane) (Math|Vector|MakeVector (.x _relativelocation) (.y _relativelocation) -8e+01) 1.0) false false))

(event EventTick
  (params (DeltaSeconds :type Float%20%28single-precision%29)))

(event EventBeginPlay
  (CallFunction|ResetPictures))

(fn ConstructionScript)