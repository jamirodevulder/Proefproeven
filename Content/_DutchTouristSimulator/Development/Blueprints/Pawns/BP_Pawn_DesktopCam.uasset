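; Desktop player character with mouse-and-keyboard walking, sprinting, free look and a photo camera aimed with the right mouse button.
; On BeginPlay the spring arm attaches to the mesh's head socket and the photo camera to the view camera.
; A visibility line trace from the camera feeds inherited functions for highlighting and HUD color each Tick, and for selection on Fire.
; Sprint doubles max walk speed while held.
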(event EventBeginPlay
  (Transformation|AttachComponentToComponent (Variables|Default|GetSpringArm) (Variables|Character|GetMesh) "head" "KeepWorld" "KeepWorld" "KeepWorld" true)
  (Transformation|AttachComponentToComponent (Variables|Default|GetPhotoCamera) (Variables|Default|GetCamera) "None" "KeepWorld" "KeepWorld" "KeepWorld" true))

(event EventTick
  (params (DeltaSeconds :type Float%20%28single-precision%29))
  ;[1 1 1] Update the highlight, the hud color and the physics handle location;
  (|CallParentFunction DeltaSeconds)
  (Utilities|IsValid (Game|GetPlayerController 0)
    (:Is%20Valid
      (bind _out_hit (CallFunction|TraceforMouse))
      (CallFunction|TrytoHighlight _out_hit)
      (CallFunction|UpdateHUDColor _out_hit))))

(event Input|ActionEvents|InputActionFire
  (params (Key :type Key%20Structure :default "None"))
  ;[1 1 1] Tries to select an object when the fire button is pressed
  (:Pressed
    (bind _out_hit (CallFunction|TraceforMouse))
    (CallFunction|TrytoSelect _out_hit)))

(event Input|ActionEvents|InputActionSprint
  (params (Key :type Key%20Structure :default "None"))
  (bind _charactermovement (Variables|Character|GetCharacterMovement))
  ;[1 1 1] Player Movement
  ;;[1 1 1] Increase Movement Speed
  (:Pressed
    (Variables|/Script/Engine.CharacterMovementComponent|SetMaxWalkSpeed _charactermovement (* (Variables|/Script/Engine.CharacterMovementComponent|GetMaxWalkSpeed _charactermovement) 2.0)))
  (:Released
    (Variables|/Script/Engine.CharacterMovementComponent|SetMaxWalkSpeed _charactermovement (/ (Variables|/Script/Engine.CharacterMovementComponent|GetMaxWalkSpeed _charactermovement) 2.0))))

(event Input|AxisEvents|InputAxisMoveForward
  (params (AxisValue :type Float%20%28single-precision%29))
  ;[1 1 1] Player Movement
  ;;[1 1 1] Movement for moving forward or backwards
  (Pawn|Input|AddMovementInput (Math|Vector|GetForwardVector (Variables|Default|GetCapsuleComponent)) (* AxisValue (Variables|Default|GetMovement%20Speed) (Utilities|Time|GetWorldDeltaSeconds)) false))

(event Input|AxisEvents|InputAxisMoveRight
  (params (AxisValue :type Float%20%28single-precision%29))
  ;[1 1 1] Player Movement
  ;;[1 1 1] Movement for moving right and left
  (Pawn|Input|AddMovementInput (Math|Vector|GetRightVector (Variables|Default|GetCapsuleComponent)) (* AxisValue (Variables|Default|GetMovement%20Speed) (Utilities|Time|GetWorldDeltaSeconds)) false))

(event Input|AxisEvents|InputAxisTurn
  (params (AxisValue :type Float%20%28single-precision%29))
  ;[1 1 1] Player Movement
  ;;[1 1 1] Handle rotation. Only rotate when the right mousebutton is pressed
  (Pawn|Input|AddControllerYawInput (* AxisValue (.x (Variables|Default|GetMouse%20Sensitivity)) (Utilities|Time|GetWorldDeltaSeconds))))

(event Input|AxisEvents|InputAxisLookUp
  (params (AxisValue :type Float%20%28single-precision%29))
  ;[1 1 1] Player Movement
  ;;[1 1 1] Handle rotation. Only rotate when the right mousebutton is pressed
  (Pawn|Input|AddControllerPitchInput (* AxisValue (.y (Variables|Default|GetMouse%20Sensitivity)) (Utilities|Time|GetWorldDeltaSeconds))))

(event Input|MouseEvents|RightMouseButton
  (params (Key :type Key%20Structure :default "None"))
  (:Pressed
    (Default|AimtheCamera (Variables|Default|GetPhotoCamera))))

(fn ConstructionScript
  (|CallParentFunction))

(fn TraceforMouse
  (bind _camera (Variables|Default|GetCamera))
  (bind _returnvalue (Transformation|GetWorldLocation _camera))
  (bind _outhit (Collision|LineTraceByChannel _returnvalue (+ (* (Math|Vector|GetForwardVector (Transformation|GetWorldRotation _camera)) 5e+03) _returnvalue) "TraceTypeQuery1" false 0 "None"))
  (return _outhit))