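; Base pawn for the Dutch Tourist Simulator that provides hit-result-driven selection and highlighting, and quits the game on Escape.
; TryToSelect and TryToHighlight forward a supplied hit to eligible Comp_Select components on the hit actor.
; UpdateHUDColor turns the player controller's HUD red over selectable components, using a DoOnce to restore the default once when blocking hits stop.
; The file performs no traces itself.
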(event Input|KeyboardEvents|Escape
  (params (Key :type Key%20Structure :default "None"))
  (:Pressed
    (Game|QuitGame 0 "Quit" false)))

(fn ConstructionScript)

(fn TrytoSelect
  (params (Hit%20Result :type Hit%20Result%20Structure))
  (bind (_bblockinghit _binitialoverlap _time _distance _location _impactpoint _normal _impactnormal _physmat _hitactor _hitcomponent) (Collision|BreakHitResult Hit%20Result))
  (if _bblockinghit
    (Utilities|IsValid _hitactor
      (:Is%20Valid
        (for _array_element (Actor|GetComponentsByClass _hitactor "/Game/_DutchTouristSimulator/Development/Blueprints/Components/Utility/Comp_Select.Comp_Select_C")
          (bind _can_be_selected (Default|CanbeSelected _array_element _hitcomponent))
          (if _can_be_selected
            (Default|SelectPressed _array_element self _location _hitcomponent)))))))

(fn TrytoHighlight
  (params (Hit%20Result :type Hit%20Result%20Structure))
  (bind (_bblockinghit _binitialoverlap _time _distance _location _impactpoint _normal _impactnormal _physmat _hitactor _hitcomponent) (Collision|BreakHitResult Hit%20Result))
  (if _bblockinghit
    (Utilities|IsValid _hitactor
      (:Is%20Valid
        (for _array_element (Actor|GetComponentsByClass _hitactor "/Game/_DutchTouristSimulator/Development/Blueprints/Components/Utility/Comp_Select.Comp_Select_C")
          (bind _can_be_selected (Default|CanbeSelected _array_element _hitcomponent))
          (if _can_be_selected
            (Default|SelectHighlight _array_element self _location (Math|Rotator|MakeRotfromZ _impactnormal) _hitcomponent)))))))

(fn UpdateHUDColor
  (params (Hit%20Result :type Hit%20Result%20Structure))
  (bind (_bblockinghit _binitialoverlap _time _distance _location _impactpoint _normal _impactnormal _physmat _hitactor _hitcomponent) (Collision|BreakHitResult Hit%20Result))
  (bind _returnvalue (Actor|GetComponentbyClass _hitactor "/Game/_DutchTouristSimulator/Development/Blueprints/Components/Utility/Comp_Select.Comp_Select_C"))
  (if _bblockinghit
    (Utilities|FlowControl|Sequence
      (:then_0
        (Utilities|FlowControl|Sequence
          (:then_0
            (Utilities|IsValid _returnvalue
              (:Is%20Valid
                (if (Utilities|Array|ContainsItem (Default|GetSelectableComponents _returnvalue) _hitcomponent)
                  (LocalVariables|SetColor%20To%20Set "(R=1.000000,G=0.000000,B=0.000000,A=1.000000)")
                  (else
                    (LocalVariables|SetUse%20Default true))))))
          (:then_1
            (bind _asbp_player_controller_main (Utilities|Casting|CastToBP_PlayerController_Main (Game|GetPlayerController 0) :!label _label))
            (Default|UpdateHUDColor _asbp_player_controller_main (LocalVariables|GetColor%20To%20Set) (LocalVariables|GetUse%20Default)))))
      (:then_1
        (goto _label_2 Reset)))
    (else
      (Utilities|FlowControl|DoOnce false :!label _label_2
        (:Completed
          (LocalVariables|SetUse%20Default true)
          (goto _label))))))