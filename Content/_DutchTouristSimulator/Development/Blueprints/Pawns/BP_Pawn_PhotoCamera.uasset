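; Player pawn for the Dutch tourist simulator that carries a photo camera as a child actor and takes pictures.
; Holding right mouse aims the camera, slows walking and enables shooting, while Fire traces for selection and takes a picture when aimed.
; The camera's picture-taken event updates the photo count on the desktop HUD component.
; When the HUD timer finishes, the game instance switches level with a fade to the quiz.
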(event TimerFinished(Comp_HUD_Desktop)
  (bind _self self)
  ;[1 1 1] Switch to quiz
  (bind _game_instance (CallFunction|GetMainGameInstance _self))
  (Default|SwitchLevel _game_instance (CallFunction|GetMapInfo _self) true))

(event Custom|On%20Picture%20Taken
  (params (Picture :type Texture%20Render%20Target%202D%20Object%20Reference) (Index :type Integer) (Photo%20Camera%20Reference :type BP%20Photo%20Camera%20Object%20Reference))
  ;[1 1 1] Update the HUD content when a picture is taken
  (Default|UpdateHUD (Variables|Default|GetComp_HUD_Desktop) (+ Index 1) -1 -1.0))

(event EventBeginPlay
  ;[1 1 1] Set the camera variable
  (|CallParentFunction)
  (bind _asbp_photo_camera (Utilities|Casting|CastToBP_PhotoCamera (Variables|/Script/Engine.ChildActorComponent|GetChildActor (Variables|Default|GetChildActor))))
  (bind _output_get (Variables|Internal|SetPhotoCamera _asbp_photo_camera))
  (Default|UpdateHUD (Variables|Default|GetComp_HUD_Desktop) -1 (Default|GetMaximumAmountOfPictures _output_get) -1.0)
  (EventDispatchers|BindEventtoOnPictureTaken _output_get (delegate Custom|On%20Picture%20Taken))
  (Components|Activation|SetActive (Variables|/Script/Engine.SceneCapture2D|GetCaptureComponent2D _output_get) false false)
  (bind _photocamera (Variables|Internal|GetPhotoCamera)
    (:then
      (Default|IdletheCamera _photocamera)
      (Variables|Internal|SetPictureAllowedToMake false))
    (:else)))

(event Input|ActionEvents|InputActionFire
  (params (Key :type Key%20Structure :default "None"))
  ;[1 1 1] Tries to select an object when the fire button is pressed
  (:Pressed
    (bind _out_hit (CallFunction|TraceforMouse))
    (CallFunction|TrytoSelect _out_hit)
    ;[1 1 1] Tries to take a picture when the fire button is pressed
    (if (Variables|Internal|GetPictureAllowedToMake)
      (bind _photocamera (Variables|Internal|GetPhotoCamera)
        (:then
          (Default|TakePicture _photocamera))
        (:else)))))

(event Input|MouseEvents|RightMouseButton
  (params (Key :type Key%20Structure :default "None"))
  (bind _charactermovement (Variables|Character|GetCharacterMovement))
  ;[1 1 1] Aim the camera and reduce movement speed when the button is pressed
  (:Pressed
    (bind _photocamera (Variables|Internal|GetPhotoCamera)
      (:then
        (Default|AimtheCamera _photocamera)
        (Variables|Internal|SetPictureAllowedToMake true)
        (Variables|/Script/Engine.CharacterMovementComponent|SetMaxWalkSpeed _charactermovement 1.5e+02))
      (:else)))
  (:Released
    (bind _photocamera_2 (Variables|Internal|GetPhotoCamera)
      (:then
        (Default|IdletheCamera _photocamera_2)
        (Variables|Internal|SetPictureAllowedToMake false)
        (Variables|/Script/Engine.CharacterMovementComponent|SetMaxWalkSpeed _charactermovement 6e+02))
      (:else))))

(fn ConstructionScript
  (|CallParentFunction))